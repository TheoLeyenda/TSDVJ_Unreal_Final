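; Pac-Man pawn Blueprint that switches between normal movement and a temporary power-up boost.
; ApplyPowerUpMovement sets the FloatingPawnMovement max speed and acceleration to power-up values, then fires the PowerUpEffect event.
; That event hosts the latent Delay for PowerUpDuration, then calls ApplyNormalMovement to restore normal values.
; Nothing in these graphs calls ApplyPowerUpMovement or handles input.
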(event Custom|Power%20Up%20Effect
  (Utilities|FlowControl|Delay (Variables|Default|GetPower%20Up%20Duration))
  (CallFunction|ApplyNormalMovement))

(fn ConstructionScript)

(fn ApplyNormalMovement
  (bind _floatingpawnmovement (Variables|Default|GetFloatingPawnMovement))
  (Utilities|FlowControl|Sequence
    (:then_0
      (Variables|/Script/Engine.FloatingPawnMovement|SetMaxSpeed _floatingpawnmovement (Variables|Default|GetNormal%20Speed)))
    (:then_1
      (Variables|/Script/Engine.FloatingPawnMovement|SetAcceleration _floatingpawnmovement (Variables|Default|GetNormal%20Aceleration)))))

(fn ApplyPowerUpMovement
  (bind _floatingpawnmovement (Variables|Default|GetFloatingPawnMovement))
  (Utilities|FlowControl|Sequence
    (:then_0
      (Variables|/Script/Engine.FloatingPawnMovement|SetMaxSpeed _floatingpawnmovement (Variables|Default|GetPowerUp%20Speed)))
    (:then_1
      (Variables|/Script/Engine.FloatingPawnMovement|SetAcceleration _floatingpawnmovement (Variables|Default|GetPower%20Up%20Aceleration)))
    (:then_2
      (CallFunction|PowerUpEffect))))